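; Board actor that builds a path of tile meshes at BeginPlay from its Tiles array.
; The first tile uses its own position; later ones step 300 units by authored direction or, in RandomMode, via RandomChoice.
; RandomChoice re-rolls on positions in ArrayOfUsedPositions, which omits the first tile, and has no retry limit.
; Each tile gets its mesh and a neutral, positive or negative material from IntType and MovementChange.
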(event Custom|RandomChoice
  (bind _randomintceiling (Variables|Default|GetRandomIntCeiling))
  (bind _randomintfloor (Variables|Default|GetRandomIntFloor))
  (bind _previousmeshlocation (Variables|Default|GetPreviousMeshLocation))
  (bind _previousmeshlocation_2 (Variables|Default|GetPreviousMeshLocation))
  (bind _previousmeshlocation_3 (Variables|Default|GetPreviousMeshLocation))
  (bind _previousmeshlocation_4 (Variables|Default|GetPreviousMeshLocation))
  (bind _returnvalue (Math|Random|RandomIntegerinRange _randomintfloor _randomintceiling))
  (switch int _returnvalue :!label _label
    (:0
      (bind _output_get (Variables|Default|SetExcludedInt 1))
      (if (== _returnvalue _output_get)
        (goto _label)
        (else
          (bind _output_get_2 (Variables|Default|SetNewMeshLocation (Math|Vector|MakeVector (.x _previousmeshlocation_4) (+ (.y _previousmeshlocation_4) -3e+02) (.z _previousmeshlocation_4))))
          (Variables|Default|SetNewMeshLocation _output_get_2))))
    (:1
      (bind _output_get_3 (Variables|Default|SetExcludedInt 0))
      (if (== _returnvalue _output_get_3)
        (goto _label)
        (else
          (bind _output_get_4 (Variables|Default|SetNewMeshLocation (Math|Vector|MakeVector (.x _previousmeshlocation_2) (+ (.y _previousmeshlocation_2) 3e+02) (.z _previousmeshlocation_2))))
          (Variables|Default|SetNewMeshLocation _output_get_4))))
    (:2
      (bind _output_get_5 (Variables|Default|SetExcludedInt 3))
      (if (== _returnvalue _output_get_5)
        (goto _label)
        (else
          (bind _output_get_6 (Variables|Default|SetNewMeshLocation (Math|Vector|MakeVector (+ (.x _previousmeshlocation_3) 3e+02) (.y _previousmeshlocation_3) (.z _previousmeshlocation_3))))
          (Variables|Default|SetNewMeshLocation _output_get_6))))
    (:3
      (bind _output_get_7 (Variables|Default|SetExcludedInt 2))
      (if (== _returnvalue _output_get_7)
        (goto _label)
        (else
          (bind _output_get_8 (Variables|Default|SetNewMeshLocation (Math|Vector|MakeVector (+ (.x _previousmeshlocation) -3e+02) (.y _previousmeshlocation) (.z _previousmeshlocation))))
          (Variables|Default|SetNewMeshLocation _output_get_8)))))
  (Variables|Default|SetBreaked false)
  (bind _array_element (Utilities|Array|ForEachLoopwithBreak (Variables|Default|GetArrayOfUsedPositions) :!label _label_2)
    (:LoopBody
      (if (Utilities|Operators|EqualEqual _array_element (Variables|Default|GetNewMeshLocation) 0.0)
        (Variables|Default|SetBreaked true)
        (goto _label_2 Break)))
    (:Completed
      (if (Variables|Default|GetBreaked)
        (goto _label)))))

(event EventBeginPlay
  (Utilities|Array|Clear (Variables|Default|GetArrayOfUsedPositions))
  (for (_array_element _array_index) (Variables|Default|GetTiles)
    (if (== _array_index 0)
      (bind _returnvalue (AddComponent|AddStaticMeshComponent false (Math|Transform|MakeTransform (.Position (Utilities|Struct|BreakST_Tiles _array_element)) "0, 0, 0" "1.000000,1.000000,1.000000")))
      (Variables|Default|SetCurrentTileMesh _returnvalue)
      (else
        (if (Variables|Default|GetRandomMode)
          (CallFunction|RandomChoice)
          (else
            (switch Utilities|FlowControl|Switch|SwitchonE_TilePositions (.Enum (Utilities|Struct|BreakST_Tiles _array_element))
              (:NewEnumerator0
                (bind _output_get (Variables|Default|SetNewMeshLocation (Math|Vector|MakeVector (.x (Variables|Default|GetPreviousMeshLocation)) (+ (.y (Variables|Default|GetPreviousMeshLocation)) -3e+02) (.z (Variables|Default|GetPreviousMeshLocation)))))
                (Variables|Default|SetNewMeshLocation _output_get))
              (:NewEnumerator1
                (bind _output_get_2 (Variables|Default|SetNewMeshLocation (Math|Vector|MakeVector (.x (Variables|Default|GetPreviousMeshLocation)) (+ (.y (Variables|Default|GetPreviousMeshLocation)) 3e+02) (.z (Variables|Default|GetPreviousMeshLocation)))))
                (Variables|Default|SetNewMeshLocation _output_get_2))
              (:NewEnumerator2
                (bind _output_get_3 (Variables|Default|SetNewMeshLocation (Math|Vector|MakeVector (+ (.x (Variables|Default|GetPreviousMeshLocation)) 3e+02) (.y (Variables|Default|GetPreviousMeshLocation)) (.z (Variables|Default|GetPreviousMeshLocation)))))
                (Variables|Default|SetNewMeshLocation _output_get_3))
              (:NewEnumerator3
                (bind _output_get_4 (Variables|Default|SetNewMeshLocation (Math|Vector|MakeVector (+ (.x (Variables|Default|GetPreviousMeshLocation)) -3e+02) (.y (Variables|Default|GetPreviousMeshLocation)) (.z (Variables|Default|GetPreviousMeshLocation)))))
                (Variables|Default|SetNewMeshLocation _output_get_4)))))
        (bind _returnvalue_2 (AddComponent|AddStaticMeshComponent false (Math|Transform|MakeTransform (Variables|Default|GetNewMeshLocation) "0, 0, 0" "1.000000,1.000000,1.000000")))
        (Variables|Default|SetCurrentTileMesh _returnvalue_2)
        (Utilities|Array|Add (Variables|Default|GetArrayOfUsedPositions) (Variables|Default|GetNewMeshLocation))))
    (Components|StaticMesh|SetStaticMesh (Variables|Default|GetCurrentTileMesh) (.Mesh (Utilities|Struct|BreakST_Tiles _array_element)))
    (switch int (.IntType (Utilities|Struct|BreakST_Tiles _array_element))
      (:Default
        (Rendering|Material|SetMaterial (Variables|Default|GetCurrentTileMesh) 0 "/Game/Blueprints/Materials/M_Neutral.M_Neutral" :!label _label))
      (:0
        (goto _label))
      (:1
        (switch int (.MovementChange (Utilities|Struct|BreakST_Tiles _array_element))
          (:Default
            (Rendering|Material|SetMaterial (Variables|Default|GetCurrentTileMesh) 0 "/Game/Blueprints/Materials/M_Positive.M_Positive" :!label _label_2))
          (:0
            (goto _label_2))
          (:1
            (Rendering|Material|SetMaterial (Variables|Default|GetCurrentTileMesh) 0 "/Game/Blueprints/Materials/M_Negative.M_Negative")))))
    (Variables|Default|SetPreviousMeshLocation (Variables|Default|GetNewMeshLocation))))

(fn ConstructionScript)