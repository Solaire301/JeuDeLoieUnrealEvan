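; Player pawn for a tile-based board game that rolls a six-sided die on the D key and advances that many tiles.
; It steps through the Board's tile array one index at a time, using a timeline to lerp between tile locations with a short pause between steps.
; Landing on a Move tile starts another move by that tile's MovementChange, which can send the player backwards.
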(event Custom|GetDestination
  (params (Value :type Integer))
  (Variables|Default|SetMovementValue Value)
  (if (< (Variables|Default|GetMovementValue) 0)
    (Variables|Default|SetGoingBack true)
    (else
      (Variables|Default|SetGoingBack false)))
  (Variables|Default|SetLocationToGoInt (+ (Variables|Default|GetCurrentLocationInt) (Variables|Default|GetMovementValue)))
  (CallFunction|IncrementalMove))

(event Custom|IncrementalMove
  (bind _currentlocationint (Variables|Default|GetCurrentLocationInt))
  (if (Variables|Default|GetGoingBack) :!label _label
    (Math|Integer|DecrementInt _currentlocationint
      (:%20%20
        _))
    (else
      (Math|Integer|IncrementInt _currentlocationint
        (:%20%20
          _))))
  (Variables|Default|SetCurrentLocation (Transformation|GetActorLocation))
  (Utilities|IsValid (Utilities|Array|Get(acopy) (Variables|Default|GetTiles) (Variables|Default|GetCurrentLocationInt))
    (:Is%20Valid
      (Variables|Default|SetLocationToGo (Transformation|GetActorLocation (Utilities|Array|Get(acopy) (Variables|Default|GetTiles) (Variables|Default|GetCurrentLocationInt))))
      (bind _movement (Timeline|MoveFromTile PlayFromStart)
        (:Update
          (Transformation|SetActorLocation (Math|Vector|Lerp(Vector) (Variables|Default|GetCurrentLocation) (Variables|Default|GetLocationToGo) _movement) false false))
        (:Finished
          (Variables|Default|SetCurrentLocation (Transformation|GetActorLocation))
          (if (== (Variables|Default|GetCurrentLocationInt) (Variables|Default|GetLocationToGoInt))
            (CallFunction|IncrementalMovementEnded)
            (else
              (Utilities|FlowControl|Delay 0.5)
              (goto _label))))))))

(event Custom|IncrementalMovementEnded
  (bind _currentlocationint (Variables|Default|GetCurrentLocationInt))
  (bind _tiles (Variables|Default|GetTiles))
  (bind _output (Utilities|Array|Get(acopy) _tiles _currentlocationint))
  (switch Utilities|FlowControl|Switch|SwitchonE_TileTypes (Variables|/Game/Blueprints/BP_Tile.BP_Tile_C|GetTileType _output)
    (:NewEnumerator0
      (CallFunction|GetDestination (Variables|/Game/Blueprints/BP_Tile.BP_Tile_C|GetMovementChange _output)))))

(event Custom|RandomNumber
  (Variables|Default|SetMovementValue (Math|Random|RandomIntegerinRange 1 6))
  (Development|PrintString "Resultat du dé")
  (Development|PrintString (Utilities|String|ToString(Integer) (Variables|Default|GetMovementValue)))
  (CallFunction|GetDestination (Variables|Default|GetMovementValue)))

(event EventBeginPlay
  (Development|PrintString "play")
  (Variables|Default|SetTiles (Variables|/Game/Blueprints/BP_BoardTiles.BP_BoardTiles_C|GetTiles (Variables|Default|GetBoard)))
  (Variables|Default|SetCurrentLocationInt 0))

(event Input|KeyboardEvents|D
  (params (Key :type Key%20Structure :default "None"))
  (:Pressed
    (CallFunction|RandomNumber)))

(fn ConstructionScript)